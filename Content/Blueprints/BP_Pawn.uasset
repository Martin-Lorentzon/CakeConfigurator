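; Player pawn for a cake customizer that creates the GUI widget, yaws the camera from look input and smoothly zooms a spring arm whose height follows its length.
; Tick tracks mouse inactivity; after a few idle seconds an attract mode slowly orbits the view, slides UI panels away and cycles four preset cakes.
; Presets drive the GUI sliders through CakeFromValues, then the widget refreshes the cake; activity slides the panels back.
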(event Custom|UpdateIdleCake
  (bind _guiref (Variables|Default|GetGUIRef))
  (Math|Float|CompareFloat (Variables|Default|GetCakeTimer) 1.0
    (:>
      _)
    (:==
      _))
  (Variables|Default|SetCakeTimer 0.0)
  (bind _output_get (Variables|Default|SetActiveCakeExample (Class|KismetMathLibrary|Wrap (+ (Variables|Default|GetActiveCakeExample) 1) 0 4)))
  (switch int _output_get
    (:1
      (|Cake1))
    (:2
      (|Cake2))
    (:3
      (|Cake3))
    (:4
      (|Cake4)))
  (Default|UpdateStaticDetail _guiref)
  (Default|UpdateCakeColor _guiref)
  (Default|UpdateCakeHeight _guiref)
  (Default|UpdateCakeRadius _guiref))

(event Input|EnhancedActionEvents|EnhancedInputActionCustomZoomIn
  (params (ActionValue :type Boolean) (ElapsedSeconds :type Float%20%28double-precision%29) (TriggeredSeconds :type Float%20%28double-precision%29) (InputAction :type Input%20Action%20Object%20Reference :default "/Game/Inputs/CustomZoomIn.CustomZoomIn"))
  ;[0.7016 1 0] Process Zoom(Scroll wheel) Input
  (:Triggered
    (Variables|Default|SetArmLength (Math|Float|Clamp(Float) (- (Variables|Default|GetArmLength) 25.0) 6e+01 2e+02))))

(event Input|EnhancedActionEvents|EnhancedInputActionCustomMouseLook
  (params (ActionValue :type Vector%202D%20Structure) (ElapsedSeconds :type Float%20%28double-precision%29) (TriggeredSeconds :type Float%20%28double-precision%29) (InputAction :type Input%20Action%20Object%20Reference :default "/Game/Inputs/CustomMouseLook.CustomMouseLook"))
  (:Triggered
    (Pawn|Input|AddControllerYawInput (.x ActionValue))))

(event Input|EnhancedActionEvents|EnhancedInputActionCustomZoomOut
  (params (ActionValue :type Boolean) (ElapsedSeconds :type Float%20%28double-precision%29) (TriggeredSeconds :type Float%20%28double-precision%29) (InputAction :type Input%20Action%20Object%20Reference :default "/Game/Inputs/CustomZoomOut.CustomZoomOut"))
  ;[0.7016 1 0] Process Zoom(Scroll wheel) Input
  (:Triggered
    (Variables|Default|SetArmLength (Math|Float|Clamp(Float) (+ (Variables|Default|GetArmLength) 25.0) 6e+01 2e+02))))

(event EventBeginPlay
  (bind _returnvalue (Game|GetPlayerController 0))
  (bind _uipanels (Variables|Default|GetUIPanels))
  ;[1 0 0.7033] Add Mapping Context
  (bind _asplayer_controller (Utilities|Casting|CastToPlayerController (Pawn|GetController)))
  (Input|AddMappingContext (PlayerController|LocalPlayerSubsystems|GetEnhancedInputLocalPlayerSubsystem _asplayer_controller) "/Game/Inputs/MyInputMappingContext.MyInputMappingContext" 0 "(bIgnoreAllPressedKeysUntilRelease=True,bForceImmediately=False)")
  (bind _returnvalue_2 (UserInterface|CreateWidget "/Game/Blueprints/GUIWidget.GUIWidget_C"))
  (bind _output_get (Variables|Default|SetGUIRef _returnvalue_2))
  (UserInterface|Viewport|AddtoViewport _output_get 0)
  (Input|SetInputModeGameandUI _returnvalue _output_get "DoNotLock" true false)
  (Variables|/Script/Engine.PlayerController|SetbShowMouseCursor _returnvalue true)
  (Utilities|Array|SetArrayElem _uipanels 0 (Variables|/Game/Blueprints/GUIWidget.GUIWidget_C|GetCakeVBox (Variables|Default|GetGUIRef)) true)
  (Utilities|Array|SetArrayElem _uipanels 1 (Variables|/Game/Blueprints/GUIWidget.GUIWidget_C|GetStrawberriesVBox (Variables|Default|GetGUIRef)) true)
  (Utilities|Array|SetArrayElem _uipanels 2 (Variables|/Game/Blueprints/GUIWidget.GUIWidget_C|GetCreamVBox (Variables|Default|GetGUIRef)) true)
  (Utilities|Array|SetArrayElem _uipanels 3 (Variables|/Game/Blueprints/GUIWidget.GUIWidget_C|GetCherriesVBox (Variables|Default|GetGUIRef)) true)
  (Utilities|Array|SetArrayElem _uipanels 4 (Variables|/Game/Blueprints/GUIWidget.GUIWidget_C|GetCookiesVBox (Variables|Default|GetGUIRef)) true))

(event Collision|EventActorBeginOverlap
  (params (OtherActor :type Actor%20Object%20Reference)))

(event EventTick
  (params (DeltaSeconds :type Float%20%28single-precision%29))
  (bind _returnvalue (Game|GetPlayerController 0))
  (bind (_locationx _locationy) (Game|Player|GetMousePosition _returnvalue))
  ;[0 0.8444 1] Interpolate Target Arm Length
  (bind _output_get (Variables|/Script/Engine.SpringArmComponent|SetTargetArmLength (Variables|Default|GetSpringArm) (Math|Float|Lerp (Variables|/Script/Engine.SpringArmComponent|GetTargetArmLength (Variables|Default|GetSpringArm)) (Variables|Default|GetArmLength) (* DeltaSeconds 8.0))))
  ;[0 0.4322 1] Adjust Arm Height
  (Transformation|SetRelativeLocation (Variables|Default|GetSpringArm) (Math|Vector|MakeVector 0.0 0.0 (Math|Float|MapRangeClamped _output_get 6e+01 2e+02 -45.0 37.66)) false false)
  ;[0 0.1993 1] Is any MB down?
  (if (Input|EnhancedActionValues|GetCustomAnyMB)
    (Variables|Default|SetInactiveTimer 0.0)
    (else
      ;[0.05509 0 1] Add seconds to TimeInactive if mouse is stationary
      (Math|Float|CompareFloat (+ _locationx _locationy) (+ (.x (stale _output_get_2)) (.y (stale _output_get_2)))
        (:>
          (Variables|Default|SetInactiveTimer 0.0 :!label _label))
        (:==
          (Variables|Default|SetInactiveTimer (+ (Variables|Default|GetInactiveTimer) (Utilities|Time|GetWorldDeltaSeconds))))
        (:<
          (goto _label)))
      (bind _output_get_2 (Variables|Default|SetPreviousMouseXY (Math|Vector2D|MakeVector2D _locationx _locationy)))))
  (Math|Float|CompareFloat (Variables|Default|GetInactiveTimer) 8.0
    (:>
      (Variables|Default|SetInactiveCamSpeed (Math|Float|Lerp (Variables|Default|GetInactiveCamSpeed) 0.2 (* (Utilities|Time|GetWorldDeltaSeconds) 4.0)))
      (Pawn|Input|AddControllerYawInput (Variables|Default|GetInactiveCamSpeed))
      (Variables|Default|SetCakeTimer (+ (Variables|Default|GetCakeTimer) (Utilities|Time|GetWorldDeltaSeconds)))
      (CallFunction|UpdateIdleCake)
      (for _array_element (Variables|Default|GetUIPanels)
        (Variables|/Script/UMG.Widget|SetRenderTransform _array_element (Utilities|Struct|MakeWidgetTransform (Math|Vector2D|MakeVector2D 0.0 (Math|Float|Lerp (.y (.translation (Variables|/Script/UMG.Widget|GetRenderTransform _array_element))) -5e+02 (Utilities|Time|GetWorldDeltaSeconds))) "(X=1.000000,Y=1.000000)" "(X=0.000000,Y=0.000000)" 0.0))))
    (:==
      (Variables|Default|SetInactiveCamSpeed 0.0 :!label _label_2)
      (Variables|Default|SetCakeTimer 0.0)
      (for _array_element_2 (Variables|Default|GetUIPanels)
        (Variables|/Script/UMG.Widget|SetRenderTransform _array_element_2 (Utilities|Struct|MakeWidgetTransform (Math|Vector2D|MakeVector2D 0.0 (Math|Float|Lerp (.y (.translation (Variables|/Script/UMG.Widget|GetRenderTransform _array_element_2))) 0.0 (* (Utilities|Time|GetWorldDeltaSeconds) 2.0))) "(X=1.000000,Y=1.000000)" "(X=0.000000,Y=0.000000)" 0.0))))
    (:<
      (goto _label_2))))

(fn ConstructionScript)

(fn CakefromValues
  (params (Radius :type Float%20%28double-precision%29) (Height :type Float%20%28double-precision%29) (COLOR____________________ :type Boolean) (Color_R :type Float%20%28double-precision%29) (Color_G :type Float%20%28double-precision%29) (Color_B :type Float%20%28double-precision%29) (STRAWBERRIES__________ :type Boolean) (SB_Amount :type Float%20%28double-precision%29) (SB_Distance :type Float%20%28double-precision%29) (SB_Height :type Float%20%28double-precision%29) (WHIPPED_CREAM__________ :type Boolean) (WC_Amount :type Float%20%28double-precision%29) (WC_Distance :type Float%20%28double-precision%29) (WC_Height :type Float%20%28double-precision%29) (CHERRIES__________ :type Boolean) (CH_Amount :type Float%20%28double-precision%29) (CH_Distance :type Float%20%28double-precision%29) (CH_Height :type Float%20%28double-precision%29) (COOKIES__________ :type Boolean) (OR_Amount :type Float%20%28double-precision%29) (OR_Distance :type Float%20%28double-precision%29) (OR_Height :type Float%20%28double-precision%29))
  (bind _guiref (Variables|Default|GetGUIRef))
  (Class|Slider|SetValue (Variables|/Game/Blueprints/GUIWidget.GUIWidget_C|GetRadiusSlider _guiref) Radius)
  (Class|Slider|SetValue (Variables|/Game/Blueprints/GUIWidget.GUIWidget_C|GetHeightSlider _guiref) Height)
  (Class|Slider|SetValue (Variables|/Game/Blueprints/GUIWidget.GUIWidget_C|GetChannel_R_Slider _guiref) Color_R)
  (Class|Slider|SetValue (Variables|/Game/Blueprints/GUIWidget.GUIWidget_C|GetChannel_G_Slider _guiref) Color_G)
  (Class|Slider|SetValue (Variables|/Game/Blueprints/GUIWidget.GUIWidget_C|GetChannel_B_Slider _guiref) Color_B)
  (Class|Slider|SetValue (Variables|/Game/Blueprints/GUIWidget.GUIWidget_C|GetSB_AmountSlider _guiref) SB_Amount)
  (Class|Slider|SetValue (Variables|/Game/Blueprints/GUIWidget.GUIWidget_C|GetSB_DistanceSlider _guiref) SB_Distance)
  (Class|Slider|SetValue (Variables|/Game/Blueprints/GUIWidget.GUIWidget_C|GetSB_HeightSlider _guiref) SB_Height)
  (Class|Slider|SetValue (Variables|/Game/Blueprints/GUIWidget.GUIWidget_C|GetWC_AmountSlider _guiref) WC_Amount)
  (Class|Slider|SetValue (Variables|/Game/Blueprints/GUIWidget.GUIWidget_C|GetWC_DistanceSlider _guiref) WC_Distance)
  (Class|Slider|SetValue (Variables|/Game/Blueprints/GUIWidget.GUIWidget_C|GetWC_HeightSlider _guiref) WC_Height)
  (Class|Slider|SetValue (Variables|/Game/Blueprints/GUIWidget.GUIWidget_C|GetCH_AmountSlider _guiref) CH_Amount)
  (Class|Slider|SetValue (Variables|/Game/Blueprints/GUIWidget.GUIWidget_C|GetCH_DistanceSlider _guiref) CH_Distance)
  (Class|Slider|SetValue (Variables|/Game/Blueprints/GUIWidget.GUIWidget_C|GetCH_HeightSlider _guiref) CH_Height)
  (Class|Slider|SetValue (Variables|/Game/Blueprints/GUIWidget.GUIWidget_C|GetOR_AmountSlider _guiref) OR_Amount)
  (Class|Slider|SetValue (Variables|/Game/Blueprints/GUIWidget.GUIWidget_C|GetOR_DistanceSlider _guiref) OR_Distance)
  (Class|Slider|SetValue (Variables|/Game/Blueprints/GUIWidget.GUIWidget_C|GetOR_HeightSlider _guiref) OR_Height))